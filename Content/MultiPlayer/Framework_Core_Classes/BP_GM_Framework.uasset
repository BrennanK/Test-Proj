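; Multiplayer framework game mode that tracks player controllers, relays score changes and respawns players.
; Login, controller swap and logout events maintain the controller list.
; The score event loops over that list, pushing the first team's new score directly into each controller's score widget.
; SpawnPlayer destroys the controlled pawn, spawns a third-person character at a random PlayerStart, then, with authority, possesses it and calls its possession override.
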(event Custom|Update%20Scores%20across%20all%20players
  (params (New%20Score :type Integer))
  (for _array_element (Variables|Default|GetAll%20Player%20Controllers)
    (bind _asbp_pc_framework (Utilities|Casting|CastToBP_PC_Framework _array_element))
    (Utilities|IsValid (Variables|/Game/MultiPlayer/Framework_Core_Classes/BP_PC_Framework.BP_PC_Framework_C|GetScore%20widget _asbp_pc_framework)
      (:Is%20Valid
        (Default|Update1stTeamScore (Variables|/Game/MultiPlayer/Framework_Core_Classes/BP_PC_Framework.BP_PC_Framework_C|GetScore%20widget _asbp_pc_framework) New%20Score)))))

(event EventPostLogin
  (params (NewPlayer :type Player%20Controller%20Object%20Reference))
  (Utilities|Array|Add (Variables|Default|GetAll%20Player%20Controllers) NewPlayer))

(event EventOnSwapPlayerControllers
  (params (OldPC :type Player%20Controller%20Object%20Reference) (NewPC :type Player%20Controller%20Object%20Reference))
  (Utilities|Array|Add (Variables|Default|GetAll%20Player%20Controllers) NewPC))

(event EventOnLogout
  (params (ExitingController :type Controller%20Object%20Reference))
  (bind _asbp_pc_framework (Utilities|Casting|CastToBP_PC_Framework ExitingController))
  (Utilities|Array|RemoveItem (Variables|Default|GetAll%20Player%20Controllers) _asbp_pc_framework))

(fn ConstructionScript)

(fn FindRandomPlayerstart
  (bind _outactors (Actor|GetAllActorsOfClass "/Script/Engine.PlayerStart"))
  (return (Transformation|GetActorTransform (Utilities|Array|Get(acopy) _outactors (Math|Random|RandomIntegerinRange 0 (- (Utilities|Array|Length _outactors) 1))))))

(fn SpawnPlayer
  (params (Player%20Controller :type Player%20Controller%20Object%20Reference))
  (bind _returnvalue (Pawn|GetControlledPawn Player%20Controller))
  (Utilities|IsValid _returnvalue
    (:Is%20Valid
      (Actor|DestroyActor _returnvalue))
    (:Is%20Not%20Valid
      (Development|PrintString "No controlled pawn" true true "(R=0.000000,G=0.660000,B=1.000000,A=1.000000)" 12.0)))
  (bind _returnvalue_2 (Game|SpawnActorfromClass "/Game/ThirdPerson/Blueprints/BP_ThirdPersonCharacter.BP_ThirdPersonCharacter_C" (Spawning|FindRandomPlayerstart) "Undefined" "MultiplyWithRoot" 0 0))
  (Networking|SwitchHasAuthority
    (:Authority
      (Pawn|Possess Player%20Controller _returnvalue_2)
      (Class|TestCharacter|OverridePossesion _returnvalue_2 Player%20Controller))))