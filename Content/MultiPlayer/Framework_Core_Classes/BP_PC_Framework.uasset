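; BP_PC_Framework is a multiplayer player controller that handles player spawning and a RepNotify score practice setup.
; On BeginPlay, the local controller calls ServerSpawnPlayer, which asks BP_GM_Framework to spawn its player, then adds the WB_Rep_Notify_Practice score widget to the viewport.
; Space Bar calls IncreaseeScore1 on the first Rep_Notify_Score_Actor found in the level.
; A note flags the BeginPlay flow as needing a fix for the server pawn.
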(event Custom|Server%20Spawn%20Player
  ;[1 1 1] Need to fix this for Server pawn
  (bind _asbp_gm_framework (Utilities|Casting|CastToBP_GM_Framework (Game|GetGameMode)))
  (Default|SpawnPlayer _asbp_gm_framework self))

(event EventBeginPlay
  ;[1 1 1] Need to fix this for Server pawn
  (if (Pawn|IsLocalPlayerController)
    (CallFunction|ServerSpawnPlayer)
    (bind _returnvalue (UserInterface|CreateWidget "/Game/MultiPlayer/Widgets/WB_Rep_Notify_Practice.WB_Rep_Notify_Practice_C" self))
    (UserInterface|Viewport|AddtoViewport _returnvalue 0)
    (Variables|Default|SetScore%20widget _returnvalue)))

(event Input|KeyboardEvents|SpaceBar
  (params (Key :type Key%20Structure :default "None"))
  (:Pressed
    (bind _outactors (Actor|GetAllActorsOfClass "/Game/MultiPlayer/Actors/Rep_Notify_Score_Actor.Rep_Notify_Score_Actor_C"))
    (Utilities|IsValid (Utilities|Array|Get(acopy) _outactors)
      (:Is%20Valid
        (Default|IncreaseeScore1 (Utilities|Array|Get(acopy) _outactors))))))

(fn ConstructionScript)