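; BP_Replicated_Door is a multiplayer door actor that acts as a RepNotify test, with no door movement in its graphs.
; Each Box begin overlap flips Opened without an authority check, as the SwitchHasAuthority node never runs.
; OnRep_Opened calls OpenDoor or CloseDoor, which pass 1 or 0 to Update1stTeamScore on the ScoreWidget of player controller 0, cast to BP_PC_Framework.
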(event OnComponentBeginOverlap(Box)
  (params (OverlappedComponent :type Primitive%20Component%20Object%20Reference) (OtherActor :type Actor%20Object%20Reference) (OtherComp :type Primitive%20Component%20Object%20Reference) (OtherBodyIndex :type Integer) (bFromSweep :type Boolean) (SweepResult :type Hit%20Result%20Structure%20%28by%20ref%29))
  (CallFunction|ToggleDoor))

(event Custom|Toggle%20Door
  (Variables|Default|SetOpened? (not (Variables|Default|GetOpened?))))

(event Custom|Open%20Door
  (bind _asbp_pc_framework (Utilities|Casting|CastToBP_PC_Framework (Game|GetPlayerController 0)))
  (Default|Update1stTeamScore (Variables|/Game/MultiPlayer/Framework_Core_Classes/BP_PC_Framework.BP_PC_Framework_C|GetScore%20widget _asbp_pc_framework) 1))

(event Custom|Close%20Door
  (bind _asbp_pc_framework (Utilities|Casting|CastToBP_PC_Framework (Game|GetPlayerController 0)))
  (Default|Update1stTeamScore (Variables|/Game/MultiPlayer/Framework_Core_Classes/BP_PC_Framework.BP_PC_Framework_C|GetScore%20widget _asbp_pc_framework)))

(fn ConstructionScript)

(fn OnRepOpened?
  (if (Variables|Default|GetOpened?)
    (CallFunction|OpenDoor)
    (else
      (CallFunction|CloseDoor))))